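; Player Blueprint that handles jumping and tracks score and health.
; Space or the bottom gamepad face button plays a jump animation, applies an upward velocity impulse to the capsule after a delay, then resumes the looping walk animation.
; ModifyScore and ModifyHealth update values and fire change events, with health floored at a minimum that triggers death.
; GetSelfTarget returns a fixed enum value identifying the player's target type.
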(event `Key|SpaceBar`
  (params (Key :type "Key Structure"))
  (bind _skeletalmesh (`self.SkeletalMesh`))
  (:`Pressed`
    (`SkeletalMeshComponent.PlayAnimation` _skeletalmesh "/Game/Blueprints/playerModel_Anim_test_Jump.playerModel_Anim_test_Jump" false :!label _label)
    (`KismetSystemLibrary.Delay` 1.0)
    (`self.Jump Action`)
    (`KismetSystemLibrary.Delay` 1.0)
    (`SkeletalMeshComponent.PlayAnimation` _skeletalmesh "/Game/Blueprints/playerModel_Anim_test_WalkingCycle.playerModel_Anim_test_WalkingCycle" true)))

(event `Key|Gamepad_FaceButton_Bottom`
  (params (Key :type "Key Structure"))
  (:`Pressed`
    (goto _label)))

(fn `Get Self Target`
  (returns (SelfTarget :type "/Game/Blueprints/E_Target Enum"))
  (return "NewEnumerator0"))

(fn `Jump Action`
  (`PrimitiveComponent.AddImpulse` (`self.CapsuleComponent`) (0.0 0.0 700.0) "None" true))

(fn `Modify Health`
  (params (Change :type Integer))
  (returns (Health :type Integer))
  (bind _minhealth (`self.MinHealth`))
  (bind _output_get (set `self.Health` (`KismetMathLibrary.Max` (+ (`self.Health`) Change) _minhealth)))
  (set `self.HealthPrecent` (/ (`KismetMathLibrary.Conv_IntToDouble` (`self.Health`)) (`KismetMathLibrary.Conv_IntToDouble` (`self.MaxHealth`))))
  (if (<= _output_get _minhealth)
    (`self.Death`))
  (`self.HealthChange`)
  (return _output_get))

(fn `Modify Score`
  (params (Change :type Integer))
  (returns (Score :type Integer))
  (bind _output_get (set `self.Score` (+ (`self.Score`) Change)))
  (`self.ScoreChange`)
  (return _output_get))

(fn `UserConstructionScript`)