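; Game Blueprint that spawns the moving objects, collectibles or obstacles.
; On BeginPlay it binds the spawn event to an actor-removed event, so each removal triggers a new spawn.
; Each spawn randomly picks the Collectible or Obstacle class and places it at the initial X and Y, with a height drawn at random from InitialHeights.
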(event `self.ReceiveBeginPlay`
  (add `self.ActorRemoved` (delegate `Spawn Moving Object`)))

(event `Spawn Moving Object`
  (bind _returnvalue (`KismetMathLibrary.MakeTransform` (`KismetMathLibrary.MakeVector` (.x (`self.InitialPosition`)) (.y (`self.InitialPosition`)) (`KismetArrayLibrary.Array_Random` (`self.InitialHeights`)))))
  (if (`KismetMathLibrary.RandomBool`)
    (`|SpawnActorFromClass` "/Game/Blueprints/Collectible.Collectible_C" _returnvalue "Undefined" "OverrideRootScale" null null)
    (else
      (`|SpawnActorFromClass` "/Game/Blueprints/Obstacle.Obstacle_C" _returnvalue "Undefined" "OverrideRootScale" null null))))

(fn `UserConstructionScript`)