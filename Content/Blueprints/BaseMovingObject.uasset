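; Base actor for objects that move at a constant Speed each tick and recycle themselves after hitting the player or leaving bounds.
; Overlapped actors are classified through the BaseGameObject interface: Player fires PlayerHitEvent then respawns it, Out Of Bounds respawns it after a random delay.
; Respawn returns it to InitPos X/Y with a random upward Z offset within RespawnHeightOffset.
; Its own GetSelfTarget reports Undefined.
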(event `self.ReceiveBeginPlay`
  (`AIBlueprintHelperLibrary.SimpleMoveToLocation` null (`self.init_pos`)))

(event `self.ReceiveActorBeginOverlap`
  (params (OtherActor :type "Actor Object Reference"))
  (if (`KismetSystemLibrary.DoesImplementInterface` OtherActor "/Game/Blueprints/BaseGameObject.BaseGameObject_C")
    (bind _asbase_game_object (cast `/Game/Blueprints/BaseGameObject` OtherActor))
    (bind _selftarget (`self.Get Self Target` _asbase_game_object))
    (switch `/Game/Blueprints/E_Target` _selftarget
      (:`NewEnumerator0`
        (`self.PlayerHitEvent`))
      (:`NewEnumerator1`
        (`KismetSystemLibrary.Delay` (`KismetMathLibrary.RandomFloatInRange` 0.0 5.0))))
    (`self.Respawn`)))

(event `self.ReceiveTick`
  (params (DeltaSeconds :type "Float (single-precision)"))
  (`SceneComponent.K2_AddRelativeLocation` (`self.DefaultSceneRoot`) (`self.speed`) false false))

(fn `Get Self Target`
  (returns (SelfTarget :type "/Game/Blueprints/E_Target Enum"))
  (return "NewEnumerator4"))

(fn `Respawn`
  (bind _z (.z (`self.init_pos`)))
  (`self.K2_SetActorLocation` (`KismetMathLibrary.MakeVector` (.x (`self.init_pos`)) (.y (`self.init_pos`)) (`KismetMathLibrary.RandomFloatInRange` _z (+ _z (`self.RespawnHeightOffset`))))))

(fn `UserConstructionScript`)