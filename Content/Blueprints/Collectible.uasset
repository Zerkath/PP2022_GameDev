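; Collectible Blueprint that awards points to the player when hit.
; PlayerHitEvent prints a debug message, casts player character 0 to Player and passes ScoreValue to ModifyScore.
; GetSelfTarget reports a fixed enum value as the target type.
; It has no active overlap, tick or destroy logic, so the hit event must be triggered from outside these graphs.
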(event `/Game/Blueprints/BaseGameObject.PlayerHitEvent`
  (`KismetSystemLibrary.PrintString` "Collectible hit event")
  (bind _asplayer (cast `/Game/Blueprints/Player` (`GameplayStatics.GetPlayerCharacter` 0)))
  (`/Game/Blueprints/Player.Modify Score` _asplayer (`self.ScoreValue`)))

(fn `Get Self Target`
  (returns (SelfTarget :type "/Game/Blueprints/E_Target Enum"))
  (return "NewEnumerator3"))

(fn `UserConstructionScript`
  (`parent.UserConstructionScript`))